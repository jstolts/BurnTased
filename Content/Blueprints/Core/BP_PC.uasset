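; Player controller that routes tactical camera and targeting input to the player's BP_Pawn.
; On BeginPlay it adds the IMC_Tactical Enhanced Input mapping context and caches the pawn cast to BP_Pawn.
; Input actions call the pawn's rotate, zoom, movement and target-switch functions, reducing direction to a boolean.
; The controller only forwards these calls, leaving the behavior to the pawn.
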(event `self.ReceiveBeginPlay`
  (bind _returnvalue (subsystem `EnhancedInputLocalPlayerSubsystem`))
  (`/Engine/EditorBlueprintResources/StandardMacros.IsValid` _returnvalue
    (:`Is Valid`
      (`EnhancedInputSubsystemInterface.AddMappingContext` _returnvalue "/Game/IMC_Tactical.IMC_Tactical" 0 (struct))
      (bind _asbp_pawn (cast `/Game/Blueprints/Core/BP_Pawn` (`GameplayStatics.GetPlayerPawn` 0)))
      (set `self.As BP Pawn` _asbp_pawn))))

(event `EnhancedInput|/Game/IA_RotateClockwise`
  (params (ActionValue :type Boolean) (ElapsedSeconds :type "Float (double-precision)") (TriggeredSeconds :type "Float (double-precision)") (InputAction :type "InputAction Object Reference" :default "/Game/IA_RotateClockwise.IA_RotateClockwise"))
  (:`Triggered`
    (`/Game/Blueprints/Core/BP_Pawn.RotateCamera` (`self.As BP Pawn`) false)))

(event `EnhancedInput|/Game/IA_RotateCounterClock`
  (params (ActionValue :type Boolean) (ElapsedSeconds :type "Float (double-precision)") (TriggeredSeconds :type "Float (double-precision)") (InputAction :type "InputAction Object Reference" :default "/Game/IA_RotateCounterClock.IA_RotateCounterClock"))
  (:`Triggered`
    (`/Game/Blueprints/Core/BP_Pawn.RotateCamera` (`self.As BP Pawn`) true)))

(event `EnhancedInput|/Game/IA_Zoom_Out_PC`
  (params (ActionValue :type "Float (double-precision)") (ElapsedSeconds :type "Float (double-precision)") (TriggeredSeconds :type "Float (double-precision)") (InputAction :type "InputAction Object Reference" :default "/Game/IA_Zoom_Out_PC.IA_Zoom_Out_PC"))
  (:`Triggered`
    (`/Game/Blueprints/Core/BP_Pawn.Zoom` (`self.As BP Pawn`) (> ActionValue 0.0))))

(event `EnhancedInput|/Game/MoveLeft`
  (params (ActionValue :type Boolean) (ElapsedSeconds :type "Float (double-precision)") (TriggeredSeconds :type "Float (double-precision)") (InputAction :type "InputAction Object Reference" :default "/Game/MoveLeft.MoveLeft"))
  (:`Triggered`
    (`/Game/Blueprints/Core/BP_Pawn.MoveLeftRight` (`self.As BP Pawn`) true)))

(event `EnhancedInput|/Game/MoveRight`
  (params (ActionValue :type Boolean) (ElapsedSeconds :type "Float (double-precision)") (TriggeredSeconds :type "Float (double-precision)") (InputAction :type "InputAction Object Reference" :default "/Game/MoveRight.MoveRight"))
  (:`Triggered`
    (`/Game/Blueprints/Core/BP_Pawn.MoveLeftRight` (`self.As BP Pawn`) false)))

(event `EnhancedInput|/Game/MoveForward`
  (params (ActionValue :type Boolean) (ElapsedSeconds :type "Float (double-precision)") (TriggeredSeconds :type "Float (double-precision)") (InputAction :type "InputAction Object Reference" :default "/Game/MoveForward.MoveForward"))
  (:`Triggered`
    (`/Game/Blueprints/Core/BP_Pawn.MoveForward` (`self.As BP Pawn`) true)))

(event `EnhancedInput|/Game/MoveBackward`
  (params (ActionValue :type Boolean) (ElapsedSeconds :type "Float (double-precision)") (TriggeredSeconds :type "Float (double-precision)") (InputAction :type "InputAction Object Reference" :default "/Game/MoveBackward.MoveBackward"))
  (:`Triggered`
    (`/Game/Blueprints/Core/BP_Pawn.MoveForward` (`self.As BP Pawn`) false)))

(event `EnhancedInput|/Game/IA_SwitchTarget`
  (params (ActionValue :type Boolean) (ElapsedSeconds :type "Float (double-precision)") (TriggeredSeconds :type "Float (double-precision)") (InputAction :type "InputAction Object Reference" :default "/Game/IA_SwitchTarget.IA_SwitchTarget"))
  (:`Triggered`
    (`/Game/Blueprints/Core/BP_Pawn.SwitchTarget` (`self.As BP Pawn`))))

(fn `UserConstructionScript`)