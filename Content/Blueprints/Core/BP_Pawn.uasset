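; Camera pawn with movement, yaw rotation, spring-arm zoom and optional tracking of a BP_Cube actor.
; Input events set desired location, rotation and zoom, which Tick interpolates toward; zoom level also adjusts movement and rotation speed.
; While IsTracking, the cine camera turns toward the target and the pawn heads for the midpoint between desired location and target.
; Target-switching events are empty stubs.
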(event `self.ReceiveBeginPlay`
  (bind _outactors (`GameplayStatics.GetAllActorsOfClass` "/Game/Blueprints/DebugMenu/Widgets/BP_Cube.BP_Cube_C"))
  (set `self.TrackableActors` _outactors)
  (bind _returnvalue (`GameplayStatics.GetActorOfClass` "/Game/Blueprints/DebugMenu/Widgets/BP_Cube.BP_Cube_C"))
  (set `self.ActorToTrack` _returnvalue))

(event `MoveForward`
  (params (Forward :type Boolean))
  ;[1 1 1] Player and Camera Controls
  (`self.SetDesiredForwardLocation` Forward)
  (`KismetSystemLibrary.PrintString` (`KismetStringLibrary.Conv_DoubleToString` (`self.MovementSlowdownMulti`))))

(event `MoveLeftRight`
  (params (Left :type Boolean))
  ;[1 1 1] Player and Camera Controls
  (`self.SetRightLeftLocation` Left))

(event `RotateCamera`
  (params (Counter :type Boolean))
  ;[1 1 1] Player and Camera Controls
  (`self.SetDesiredRotation` Counter))

(event `Zoom`
  (params (Zoom :type Boolean))
  ;[1 1 1] Player and Camera Controls
  (`self.SetDesiredZoom` Zoom))

(event `self.ReceiveTick`
  (params (DeltaSeconds :type "Float (single-precision)"))
  ;[1 1 1] Player and Camera Controls
  (`self.SetDesiredControls` DeltaSeconds)
  (`self.Tick`))

(event `SwitchTarget`
  ;[1 1 1] Player and Camera Controls
)

(event `RemoveFromTrackableArray`
  (params (NewParam :type "Actor Object Reference"))
  (bind _trackableactors (`self.TrackableActors`))
  (bind _actortotrack (`self.ActorToTrack`))
  (bind _output (`|GetArrayItem` _trackableactors (`KismetArrayLibrary.Array_Find` _trackableactors _actortotrack)))
  ;[1 1 1] Player and Camera Controls
  (`KismetArrayLibrary.Array_RemoveItem` (`self.TrackableActors`))
  (if (== NewParam _actortotrack)
    (`/Engine/EditorBlueprintResources/StandardMacros.IsValid` _output
      (:`Is Valid`
        (set `self.ActorToTrack` _output))
      (:`Is Not Valid`
        (if (== (`KismetArrayLibrary.Array_Length` _trackableactors) 0)
          _)))))

(event `Tick`)

(event `FindLogicalSwitch`)

(fn `SetDesiredForwardLocation`
  (params (Forward :type Boolean))
  (set `self.DesiredLocation` (+ (`self.DesiredLocation`) (* (`self.GetActorForwardVector`) (* (`KismetMathLibrary.SelectFloat` 1.0 -1.0 Forward) (- (`self.MovementSpeed`) (`self.MovementSlowdownMulti`)))))))

(fn `SetDesiredRotation`
  (params (Counter :type Boolean))
  (bind (_returnvalue_roll _returnvalue_pitch _returnvalue_yaw) (`KismetMathLibrary.BreakRotator` (`self.K2_GetActorRotation`)))
  (bind _returnvalue (* (`self.DeltaTime`) (`self.RotationMultiplier`)))
  (set `self.DesiredRotation` (`KismetMathLibrary.SelectFloat` (- _returnvalue_yaw _returnvalue) (+ _returnvalue_yaw _returnvalue) Counter)))

(fn `SetDesiredZoom`
  (params (ZoomIn :type Boolean))
  (bind _returnvalue (* (`self.DeltaTime`) (`self.ZoomMultiplier`)))
  (bind _targetarmlength (`SpringArmComponent.TargetArmLength` (`self.SpringArm`)))
  (bind _returnvalue_2 (`KismetMathLibrary.FClamp` (`KismetMathLibrary.SelectFloat` (- _targetarmlength _returnvalue) (+ _targetarmlength _returnvalue) ZoomIn) 200.0 2000.0))
  (set `self.DesiredZoom` _returnvalue_2)
  (set `self.MovementSlowdownMulti` (`KismetMathLibrary.MapRangeClamped` _returnvalue_2 1500.0 500.0 1.0 15.0)))

(fn `SetRightLeftLocation`
  (params (Left :type Boolean))
  (set `self.DesiredLocation` (+ (* (`self.GetActorRightVector`) (* (`KismetMathLibrary.SelectFloat` -1.0 1.0 Left) (- (`self.MovementSpeed`) (`self.MovementSlowdownMulti`)))) (`self.DesiredLocation`))))

(fn `UserConstructionScript`)